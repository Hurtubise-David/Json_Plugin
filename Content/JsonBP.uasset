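; JsonBP is an actor Blueprint that exercises writing and reading a JSON file, with results printed as debug output.
; Every Tick, a Sequence first writes a hardcoded server name, the ID items and the Mode values to the file named by JsonFileName.
; It then reads the same file back and prints the server name, each server item and each item value with zero-duration messages.
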(event `self.ReceiveTick`
  (params (DeltaSeconds :type "Float (single-precision)"))
  (`|ExecutionSequence`
    (:`then_0`
      ;[1 1 1] Make Json File
      (`Json_PluginBPLibrary.WriteJsonFile` (`self.JsonFileName`) "LBEVR" (`self.ID`) (`self.Mode`)))
    (:`then_1`
      ;[1 1 1] Read Json File
      (bind (_server _serveritems _itemvalue) (`Json_PluginBPLibrary.ReadJsonFile` (`self.JsonFileName`)))
      (`|ExecutionSequence`
        (:`then_0`
          (`KismetSystemLibrary.PrintString` _server true true (struct :`G` 0.66 :`B` 1.0 :`A` 1.0) 0.0))
        (:`then_1`
          (for _array_element _serveritems
            (`KismetSystemLibrary.PrintString` _array_element true true (struct :`G` 0.66 :`B` 1.0 :`A` 1.0) 0.0)))
        (:`then_2`
          (for _array_element_2 _itemvalue
            (`KismetSystemLibrary.PrintString` (`KismetStringLibrary.Conv_IntToString` _array_element_2) true true (struct :`G` 0.66 :`B` 1.0 :`A` 1.0) 0.0)))))))

(fn `UserConstructionScript`)